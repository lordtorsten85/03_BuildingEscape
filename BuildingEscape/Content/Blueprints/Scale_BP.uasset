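; Scale_BP is a scale display that shows the weight value held by a referenced projectile launcher.
; Every tick, if that reference is valid, it rounds the launcher's WeightOnScales and writes the absolute value to the Number text.
; A separate NegativeOrPositive text shows a minus sign for negative rounded values and a plus sign otherwise.
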(event `self.ReceiveTick`
  (params (DeltaSeconds :type "Float (single-precision)"))
  (bind _projectilelauncherref (`self.ProjectileLauncherRef`))
  (bind _returnvalue (`KismetMathLibrary.Round` (`ProjectileLauncher.WeightOnScales` _projectilelauncherref)))
  (`/Engine/EditorBlueprintResources/StandardMacros.IsValid` _projectilelauncherref
    (:`Is Valid`
      (`TextRenderComponent.K2_SetText` (`self.Number`) (`KismetTextLibrary.Conv_IntToText` (`KismetMathLibrary.Abs_Int` _returnvalue)))
      (`TextRenderComponent.K2_SetText` (`self.NegativeOrPositive`) (select `bool` (< _returnvalue 0) :`false` "+" :`true` "-")))))

(fn `UserConstructionScript`)